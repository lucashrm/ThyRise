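; BP_ThyRise_MenuGameMode is the menu game mode that tracks the players connected to the lobby.
; Players starting in the Lobby Menu level are registered, then their menu controllers create the lobby menu and run initial setup.
; UpdateLobby, when flagged for player names, rebuilds the profile list from all connected controllers and pushes it to each one.
; Logout removes the leaving controller and triggers that same refresh.
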(event Custom|UpdateLobby
  (params (PlayerNames :type Boolean))
  (if PlayerNames
    (Utilities|Array|Clear (Variables|Default|GetALL_PlayerProfiles))
    (for _array_element (Variables|Default|GetALL_ConnectedPlayers)
      (Utilities|Array|Add (Variables|Default|GetALL_PlayerProfiles) (Variables|/Game/Framework/BP_ThyRise_MenuController.BP_ThyRise_MenuController_C|GetPlayer%20Profile%20Info _array_element)))
    (for _array_element_2 (Variables|Default|GetALL_ConnectedPlayers)
      (if PlayerNames
        (Default|UpdatePlayerNames _array_element_2 (Variables|Default|GetALL_PlayerProfiles))))))

(event EventBeginPlay)

(event EventTick
  (params (DeltaSeconds :type Float%20%28single-precision%29)))

(event EventHandleStartingNewPlayer
  (params (NewPlayer :type Player%20Controller%20Object%20Reference))
  (bind _returnvalue (Game|GetCurrentLevelName true))
  (switch string _returnvalue
    (:LobbyMenu
      (bind _asbp_thy_rise_menu_controller (Utilities|Casting|CastToBP_ThyRise_MenuController NewPlayer))
      (Utilities|Array|Add (Variables|Default|GetALL_ConnectedPlayers) _asbp_thy_rise_menu_controller)
      (Default|CreateLobbyMenu _asbp_thy_rise_menu_controller)
      (Default|InitialSetup _asbp_thy_rise_menu_controller))))

(event EventOnLogout
  (params (ExitingController :type Controller%20Object%20Reference))
  (bind _asbp_thy_rise_menu_controller (Utilities|Casting|CastToBP_ThyRise_MenuController ExitingController))
  (Utilities|Array|RemoveItem (Variables|Default|GetALL_ConnectedPlayers) _asbp_thy_rise_menu_controller)
  (CallFunction|UpdateLobby true))

(fn ConstructionScript)