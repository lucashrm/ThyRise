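; Player controller for the menus and multiplayer lobby, giving the local player a cursor with UI-only input.
; It creates and shows lobby and load screen widgets, refreshes lobby player names, and returns to MainMenu after destroying the session.
; Initial setup loads the profile from a save slot, creating it if missing, and sends it to the server, which has the menu game mode update the lobby.
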(event Custom|EndClientSession
  (|DestroySession self
    (:then
      (Game|OpenLevel(byName) "MainMenu"))))

(event Custom|CreateLoadScreen
  (CallFunction|UIShowLoadScreen))

(event Custom|CreateLobbyMenu
  (CallFunction|UIShowLobbyMenu))

(event Custom|InitialSetup
  (CallFunction|LoadSavedProfile)
  (CallFunction|ServerUpdateLobby (Variables|Default|GetPlayer%20Profile%20Info)))

(event Custom|UpdatePlayerNames
  (params (PlayerProfiles :type Array%20of%20S%20Player%20Profile%20Structures))
  (bind _wb_lobbymenu (Variables|Default|GetWB%20LobbyMenu))
  (Utilities|IsValid _wb_lobbymenu
    (:Is%20Valid
      (Default|ClearPlayerNames _wb_lobbymenu)
      (Default|UpdatePlayerNames _wb_lobbymenu PlayerProfiles))))

(event Custom|Server_UpdateLobby
  (params (PlayerProfile :type S%20Player%20Profile%20Structure))
  (Variables|Default|SetPlayer%20Profile%20Info PlayerProfile)
  (bind _asbp_thy_rise_menu_game_mode (Utilities|Casting|CastToBP_ThyRise_MenuGameMode (Game|GetGameMode)))
  (Default|UpdateLobby _asbp_thy_rise_menu_game_mode true))

(event EventTick
  (params (DeltaSeconds :type Float%20%28single-precision%29)))

(event EventBeginPlay
  (if (Pawn|IsLocalController)
    (Variables|Default|SetbShowMouseCursor true)
    (Input|SetInputModeUIOnly self 0 "DoNotLock" false)))

(fn ConstructionScript)

(fn UIShowLobbyMenu
  (Utilities|IsValid (Variables|Default|GetWB%20LobbyMenu)
    (:Is%20Valid
      _)
    (:Is%20Not%20Valid
      (bind _returnvalue (UserInterface|CreateWidget "/Game/Widget/WB_LobbyMenu.WB_LobbyMenu_C" self))
      (Variables|Default|SetWB%20LobbyMenu _returnvalue)))
  (UserInterface|Viewport|AddtoViewport (Variables|Default|GetWB%20LobbyMenu) 0))

(fn LoadSavedProfile
  (bind _returnvalue (SaveGame|DoesSaveGameExist (LocalVariables|GetLcl_SlotName)))
  (if _returnvalue
    _
    (else
      (bind _returnvalue_2 (SaveGame|CreateSaveGameObject "/Game/SavedData/SG_PlayerProfile.SG_PlayerProfile_C"))
      (SaveGame|SaveGametoSlot _returnvalue_2 (LocalVariables|GetLcl_SlotName))))
  (bind _returnvalue_3 (SaveGame|LoadGamefromSlot (LocalVariables|GetLcl_SlotName)))
  (bind _assg_player_profile (Utilities|Casting|CastToSG_PlayerProfile _returnvalue_3))
  (Variables|Default|SetPlayer%20Profile%20Info (Variables|/Game/SavedData/SG_PlayerProfile.SG_PlayerProfile_C|GetPlayerProfile _assg_player_profile))
  (return))

(fn UIShowLoadScreen
  (Viewport|RemoveAllWidgets)
  (Utilities|IsValid (Variables|Default|GetWB_LoadScreen)
    (:Is%20Valid
      _)
    (:Is%20Not%20Valid
      (bind _returnvalue (UserInterface|CreateWidget "/Game/Widget/WB_LoadScreen.WB_LoadScreen_C" self))
      (Variables|Default|SetWB_LoadScreen _returnvalue)))
  (UserInterface|Viewport|AddtoViewport (Variables|Default|GetWB_LoadScreen) 0))